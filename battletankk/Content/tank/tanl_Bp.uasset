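; Player-controllable tank Blueprint that maps input to driving, camera aim and firing.
; On BeginPlay it registers the barrel and turret components and initialises TankMovement with the left and right tracks.
; Move and turn axes pass intents to TankMovement, while the Fire action calls Fire.
; Aim axes rotate the azimuth gimbal for yaw and the spring arm for pitch, scaled by frame time.
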(event `self.ReceiveBeginPlay`
  (`self.SetBarrelRefernce` (`self.TankBarrel`))
  (`self.SetTurretRefernce` (`self.TankTurret`))
  (`TankMovementComponent.Initialise` (`self.TankMovement`) (`self.LeftTrack`) (`self.RightTrack`)))

(event `InputAxis|AimAzimuth`
  (params (AxisValue :type "Float (single-precision)"))
  ;[1 1 1] aim input binding
  (`SceneComponent.K2_AddLocalRotation` (`self.AzimuthGimbal`) (`KismetMathLibrary.MakeRotator` 0.0 0.0 (* AxisValue (`GameplayStatics.GetWorldDeltaSeconds`) 100.0)) false false))

(event `InputAxis|MoveForward`
  (params (AxisValue :type "Float (single-precision)"))
  ;[1 1 1] movement input binding
  (`TankMovementComponent.IntendMoveForward` (`self.TankMovement`) AxisValue))

(event `InputAxis|AIMELEVATION`
  (params (AxisValue :type "Float (single-precision)"))
  ;[1 1 1] aim input binding
  (`SceneComponent.K2_AddLocalRotation` (`self.SpringArm`) (`KismetMathLibrary.MakeRotator` 0.0 (* AxisValue (`GameplayStatics.GetWorldDeltaSeconds`) 100.0)) false false))

(event `InputAxis|Turn Right`
  (params (AxisValue :type "Float (single-precision)"))
  ;[1 1 1] movement input binding
  (`TankMovementComponent.IntendTurnRight` (`self.TankMovement`) AxisValue))

(event `InputAction|Fire`
  (params (Key :type "Key Structure"))
  ;[1 1 1] aim input binding
  (:`Pressed`
    (`self.Fire`)))

(fn `UserConstructionScript`)